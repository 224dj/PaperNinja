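; Player pawn with camera-relative movement, sprinting, and a coin count that is at risk while running or dying.
; A looping timer drops a coin at full sprint speed, spawning a physics pickup launched in a random direction.
; Any damage triggers one-time death: ragdoll, non-collecting capsule, all coins dropped, timed destruction.
; ObtainScroll freezes movement and prints a delayed goal message; X and C keys drop and add coins.
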(event `DropAllCoin`
  ;[1 1 1] DropAllCoin: 코인이 1개 이상 있으면 DropCoin이 반복적으로 호출된다.
  ; 0이 되면 loop를 멈춘다.
  (while (> (`self.NumOfCoins`) 0)
    (`self.DropCoin`)))

(event `ObtainScroll`
  (`CharacterMovementComponent.DisableMovement` (`self.CharacterMovement`))
  (set `self.HasScroll` true)
  (`KismetSystemLibrary.Delay` 5.0)
  (`KismetSystemLibrary.PrintString` "goal!"))

(event `Key|X`
  (params (Key :type "Key Structure"))
  (:`Pressed`
    (`self.DropCoin`)))

(event `Key|C`
  (params (Key :type "Key Structure"))
  (:`Pressed`
    (cast `/Game/Blueprint/PNPlayerPawn` (`GameplayStatics.GetPlayerPawn` 0))
    (`self.AddCoin` 1)))

(event `self.ReceiveBeginPlay`
  (set `CharacterMovementComponent.MaxWalkSpeed` (`self.GroundWalkSpeed`) (`self.CharacterMovement`))
  (`KismetSystemLibrary.K2_SetTimer` null "CheckSprintRisk" 0.5 true))

(event `self.ReceiveAnyDamage`
  (params (Damage :type "Float (single-precision)") (DamageType :type "DamageType Object Reference") (InstigatedBy :type "Controller Object Reference") (DamageCauser :type "Actor Object Reference"))
  ;[1 1 1] Death
  (`/Engine/EditorBlueprintResources/StandardMacros.DoOnce` false
    (:`Completed`
      (`|ExecutionSequence`
        (:`then_0`
          (`KismetSystemLibrary.PrintString` "Game Over!")
          (`CharacterMovementComponent.DisableMovement` (`self.CharacterMovement`))
          (`self.SetLifeSpan` 2.0)
          (`PrimitiveComponent.SetSimulatePhysics` (`self.Mesh`) true)
          ;[1 1 1] 코인을 먹거나 하는, 충돌 처리하는 캡슐의 collision을 비활성화 해서, 죽었을 때 뭔가 획득할 수 없도록 한다.
          (`PrimitiveComponent.SetCollisionProfileName` (`self.CapsuleComponent`) "spectator"))
        (:`then_1`
          (`self.DropAllCoin`))))))

(event `InputAction|Sprint`
  (params (Key :type "Key Structure"))
  (bind _charactermovement (`self.CharacterMovement`))
  ;[1 1 1] Movement
  ;;[1 1 1] Sprint & Walk
  (:`Pressed`
    (set `CharacterMovementComponent.MaxWalkSpeed` (`self.GroundSprintSpeed`) _charactermovement))
  (:`Released`
    (set `CharacterMovementComponent.MaxWalkSpeed` (`self.GroundWalkSpeed`) _charactermovement)))

(event `InputAxis|MoveForward`
  (params (AxisValue :type "Float (single-precision)"))
  ;[1 1 1] Movement
  (`self.AddMovementInput` (`/Game/Blueprint/PNFuncLibrary.Flatten Direction` (`SceneComponent.GetForwardVector` (`self.Camera`))) AxisValue) ; 앞으로 이동
)

(event `InputAxis|LookUp`
  (params (AxisValue :type "Float (single-precision)"))
  ;[1 1 1] Movement
  ;;[1 1 1] Camera
  (`self.AddControllerPitchInput` AxisValue))

(event `InputAxis|MoveRight`
  (params (AxisValue :type "Float (single-precision)"))
  ;[1 1 1] Movement
  (`self.AddMovementInput` (`/Game/Blueprint/PNFuncLibrary.Flatten Direction` (`SceneComponent.GetRightVector` (`self.Camera`))) AxisValue) ; 오른쪽 이동
)

(event `InputAxis|LookRight`
  (params (AxisValue :type "Float (single-precision)"))
  ;[1 1 1] Movement
  ;;[1 1 1] Camera
  (`self.AddControllerYawInput` AxisValue))

(fn `AddCoin`
  (params (num :type Integer))
  (set `self.NumOfCoins` (+ (`self.NumOfCoins`) num)))

(fn `CheckSprintRisk`
  (if (>= (`/Game/Blueprint/PNActorMacroLibrary.GetFlatSpeed`) (`self.GroundSprintSpeed`))
    (`self.DropCoin`)))

(fn `DropCoin`
  (if (>= (`self.NumOfCoins`) 1)
    (set `self.NumOfCoins` (- (`self.NumOfCoins`) 1))
    (bind _returnvalue (`|SpawnActorFromClass` "/Game/Blueprint/PNPickUpCoinActor.PNPickupCoinActor_C" (`SceneComponent.GetSocketTransform` (`self.Mesh`) "CoinSpawnPoint" "RTS_World") "Undefined" "OverrideRootScale" null null))
    (bind _staticmeshcomponent (`StaticMeshActor.StaticMeshComponent` _returnvalue))
    (`PrimitiveComponent.SetSimulatePhysics` _staticmeshcomponent true)
    (`PrimitiveComponent.AddImpulse` _staticmeshcomponent (`KismetMathLibrary.RotateAngleAxis` (`KismetMathLibrary.MakeVector` 200.0 0.0 200.0) (`KismetMathLibrary.RandomFloatInRange` 0.0 360.0) (0.0 0.0 1.0)) "None" true)))

(fn `GetNumOfCoins`
  (returns (ReturnValue :type Integer))
  (return (`self.NumOfCoins`)))

(fn `UserConstructionScript`)