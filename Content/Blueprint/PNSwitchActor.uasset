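; Floor switch actor that sinks its mesh when something overlaps its box trigger and signals on and off state changes.
; A timeline lerps the mesh down slightly, then calls SwitchTurnedOn or SwitchTurnedOff depending on its finish direction.
; Ending overlap reverses it only for momentary switches, while SwitchTurnedOff_Event also reverses it.
; Overlaps are unfiltered, as the Player tag check is unconnected.
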(event `self.BoxTrigger.OnComponentBeginOverlap`
  (params (OverlappedComponent :type "PrimitiveComponent Object Reference") (OtherActor :type "Actor Object Reference") (OtherComp :type "PrimitiveComponent Object Reference") (OtherBodyIndex :type Integer) (bFromSweep :type Boolean) (SweepResult :type "HitResult Structure (by ref)"))
  (bind (_direction _alpha) (`Timeline|SwitchTimeline` :!label _label)
    (:`Update`
      (`SceneComponent.K2_SetRelativeLocationAndRotation` :`self` (`self.Mesh`) :`NewLocation` (`KismetMathLibrary.VLerp` (0.0 0.0 0.0) (0.0 0.0 -8.0) _alpha)))
    (:`Finished`
      (switch `ETimelineDirection` _direction
        (:`Forward`
          (`self.SwitchTurnedOn`))
        (:`Backward`
          (`self.SwitchTurnedOff`))))))

(event `self.BoxTrigger.OnComponentEndOverlap`
  (params (OverlappedComponent :type "PrimitiveComponent Object Reference") (OtherActor :type "Actor Object Reference") (OtherComp :type "PrimitiveComponent Object Reference") (OtherBodyIndex :type Integer))
  (if (`self.IsMomentary`)
    (goto _label :!via `Reverse`)))

(event `SwitchTurnedOff_Event`
  (goto _label :!via `Reverse`))

(fn `UserConstructionScript`)